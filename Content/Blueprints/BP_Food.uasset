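; BP_Food is a food pickup that loses score value as it ages, signalled by its polygon sprite color.
; On BeginPlay it starts as Blue, the most valuable stage.
; The SetFood event switches on type to set sprite and ScoreVal, then re-calls itself after progressively shorter Delays, stepping through Purple and Red until it settles on Yellow.
; Collection and scoring are not handled in this graph.
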(event Custom|SetFood
  (params (Type :type FoodColor_Enum%20Enum :default "NewEnumerator0"))
  (bind _foodsprite (Variables|Default|GetFoodSprite))
  (switch Utilities|FlowControl|Switch|SwitchonFoodColor_Enum Type
    (:NewEnumerator0
      (Rendering|Components|Sprite|SetSprite _foodsprite "/Game/Sprites/BluePolygon_Sprite.BluePolygon_Sprite")
      (Variables|Default|SetScoreVal 100)
      (Utilities|FlowControl|Delay 3.0)
      (CallFunction|SetFood "NewEnumerator1"))
    (:NewEnumerator1
      (Rendering|Components|Sprite|SetSprite _foodsprite "/Game/Sprites/PurplePolygon_Sprite.PurplePolygon_Sprite")
      (Variables|Default|SetScoreVal 50)
      (Utilities|FlowControl|Delay 2.0)
      (CallFunction|SetFood "NewEnumerator2"))
    (:NewEnumerator2
      (Rendering|Components|Sprite|SetSprite _foodsprite "/Game/Sprites/RedPolygon_Sprite.RedPolygon_Sprite")
      (Variables|Default|SetScoreVal 20)
      (Utilities|FlowControl|Delay 1.0)
      (CallFunction|SetFood "NewEnumerator3"))
    (:NewEnumerator3
      (Rendering|Components|Sprite|SetSprite _foodsprite "/Game/Sprites/YellowPolygon_Sprite.YellowPolygon_Sprite")
      (Variables|Default|SetScoreVal 10))))

(event EventBeginPlay
  (CallFunction|SetFood "NewEnumerator0"))

(fn ConstructionScript)