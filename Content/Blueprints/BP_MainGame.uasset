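; Main actor for a grid-based 2D Snake game on the XZ plane, handling setup, scoring, HUD, game over and R-to-reload.
; BeginPlay spawns the head, food and border walls.
; A Delay on Tick paces each step: position-comparison collision checks, growth and speed-up on eating, gated WASD steering, then tail-to-head movement.
; Hitting itself or a wall swaps the snake's flipbooks, destroys it and notifies the HUD.
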(event Custom|SpawnNewSnakePart
  (params (SpawnLocation :type Vector) (IsHead :type Boolean))
  ;[1 1 1] Spawn New Snake Part
  (bind _returnvalue (Game|SpawnActorfromClass "/Game/Blueprints/BP_SnakeBodyPart.BP_SnakeBodyPart_C" (Math|Transform|MakeTransform SpawnLocation "0,0.000000, 0" "1,1,1") "AlwaysSpawn" 0 IsHead 0))
  (Sprite|SetFlipbook (Variables|/Game/Blueprints/BP_SnakeBodyPart.BP_SnakeBodyPart_C|GetPaperFlipbook _returnvalue) (select IsHead "/Game/Flipbooks/RedSquare_Flipbook.RedSquare_Flipbook" "/Game/Flipbooks/YellowSquare_Flipbook.YellowSquare_Flipbook"))
  (Utilities|Array|Add (Variables|Default|GetSnakePartsArray) _returnvalue)
  (Transformation|SetActorRotation _returnvalue (Math|Rotator|MakeRotator 0.0 (Utilities|Select :Index (Math|Random|RandomInteger 4) :Option%200 0.0 :Option%201 9e+01 :Option%202 1.8e+02 :Option%203 2.7e+02) 0.0)))

(event Custom|Spawn%20Food
  (bind _x_max (Variables|Default|GetX_Max))
  (bind _z_max (Variables|Default|GetZ_Max))
  (bind _returnvalue (- _z_max 1e+02))
  (bind _returnvalue_2 (- _x_max 1e+02))
  ;[1 1 1] Spawn Food
  (bind _returnvalue_3 (Game|SpawnActorfromClass "/Game/Blueprints/BP_Food.BP_Food_C" (Math|Transform|MakeTransform (Math|Vector|MakeVector (* (.ReturnValue (Math|Float|Division(WholeandRemainder) (Math|Random|RandomFloatinRange (* _returnvalue_2 -1.0) _returnvalue_2) 1e+02)) 1e+02) -0.1 (* (.ReturnValue (Math|Float|Division(WholeandRemainder) (Math|Random|RandomFloatinRange (* _returnvalue -1.0) _returnvalue) 1e+02)) 1e+02)) "0, 0, 0" "1,1,1") "AlwaysSpawn" 0 0))
  (Variables|Default|SetFoodActorREF _returnvalue_3))

(event Custom|Kill%20Snake
  ;[1 1 1] Kill Snake And Game Over
  (Variables|Default|SetIsDead true)
  (for (_array_element _array_index) (Variables|Default|GetSnakePartsArray)
    (Sprite|SetFlipbook (Variables|/Game/Blueprints/BP_SnakeBodyPart.BP_SnakeBodyPart_C|GetPaperFlipbook _array_element) (select (== _array_index 0) "/Game/Flipbooks/Blank_Flipbook.Blank_Flipbook" "/Game/Flipbooks/Beath_Flipbook.Beath_Flipbook")))
  (Utilities|FlowControl|Delay 0.5)
  (for _array_element_2 (Variables|Default|GetSnakePartsArray)
    (Actor|DestroyActor _array_element_2))
  (Utilities|Array|Clear (Variables|Default|GetSnakePartsArray))
  (Default|GameOverEvent (Variables|Default|GetHUD_REF)))

(event Custom|UpdateScore
  (params (Val :type Integer))
  ;[1 1 1] Update Score
  (bind _output_get (Variables|Default|SetScore (+ Val (Variables|Default|GetScore))))
  (Default|UpdateScore (Variables|Default|GetHUD_REF) _output_get))

(event EventBeginPlay
  ;[1 1 1] Initialize Game
  (|CreateHUDWidget)
  (|SelectRandomStartDirection)
  (|SetUpdateDelay)
  (|SpawnSnakeHead)
  (|SpawnFirstFood)
  (|SpawnWalls))

(event EventTick
  (params (DeltaSeconds :type Float%20%28single-precision%29))
  (if (Variables|Default|GetIsDead)
    ;[1 1 1] restart level when dead and 'R' pressed
    (Utilities|FlowControl|Gate true
      (:Exit
        (Utilities|FlowControl|DoOnce false
          (:Completed
            (Widget|RemovefromParent (Variables|Default|GetHUD_REF))
            (bind _returnvalue (Game|GetCurrentLevelName true))
            (Game|OpenLevel(byName) (Utilities|String|StringToName _returnvalue))))))
    (else
      (Utilities|FlowControl|Delay (Variables|Default|GetDelay))
      (Utilities|FlowControl|Sequence
        (:then_0
          (|GameOverIfSelfCollision))
        (:then_1
          (|GameOverIfWallCollision))
        (:then_2
          (|EatFoodIfCollision
            (:true
              (|AddSnakePart)
              (CallFunction|SpawnFood)
              (|SpeedUpSnake))))
        (:then_3
          (|ChangeDirectionOnInput
            (:out
              (|MoveSnake))))))))

(event Input|KeyboardEvents|R
  (params (Key :type Key%20Structure :default "None"))
  (:Pressed
    ;[1 1 1] restart level when dead and 'R' pressed
    (Utilities|FlowControl|Gate true) ; enters at Open
  ))

(fn ConstructionScript)

(event Input|KeyboardEvents|W
  (params (Key :type Key%20Structure :default "None"))
  (:Pressed
    (Utilities|FlowControl|Gate true) ; enters at Open
  )
  (:Released
    (Utilities|FlowControl|Gate true) ; enters at Close
  ))

(event Input|KeyboardEvents|S
  (params (Key :type Key%20Structure :default "None"))
  (:Pressed
    (Utilities|FlowControl|Gate true) ; enters at Open
  )
  (:Released
    (Utilities|FlowControl|Gate true) ; enters at Close
  ))

(event Input|KeyboardEvents|A
  (params (Key :type Key%20Structure :default "None"))
  (:Pressed
    (Utilities|FlowControl|Gate true) ; enters at Open
  )
  (:Released
    (Utilities|FlowControl|Gate true) ; enters at Close
  ))

(event Input|KeyboardEvents|D
  (params (Key :type Key%20Structure :default "None"))
  (:Pressed
    (Utilities|FlowControl|Gate true) ; enters at Open
  )
  (:Released
    (Utilities|FlowControl|Gate true) ; enters at Close
  ))

(event Custom|BreakSelfCollisionTestLoop
  (Utilities|Array|ForEachLoopwithBreak (Variables|Default|GetSnakePartsArray)) ; enters at Break
)

(event Custom|BreakWallCollisionLoop
  (Utilities|Array|ForEachLoopwithBreak (Variables|Default|GetWallBlocksArray)) ; enters at Break
)